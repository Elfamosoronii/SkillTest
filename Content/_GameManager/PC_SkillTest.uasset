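; PC_SkillTest is a player controller that turns Enhanced Input actions into movement of the controlled character.
; On possess it adds the IMC_Input mapping context.
; Move input drives the pawn along forward and right vectors from the control rotation with pitch zeroed.
; Crouch toggles on press, while sprint is held, switching max walk speed between the SprintSpeed and RunSpeed values of BP_BaseCharacter.
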(event Input|EnhancedActionEvents|EnhancedInputActionIA_Crouch
  (params (ActionValue :type Boolean) (ElapsedSeconds :type Float%20%28double-precision%29) (TriggeredSeconds :type Float%20%28double-precision%29) (InputAction :type Input%20Action%20Object%20Reference :default "/Game/_GameManager/Input/IA_Crouch.IA_Crouch"))
  (bind _returnvalue (Pawn|GetControlledPawn))
  (bind _ascharacter (Utilities|Casting|CastToCharacter _returnvalue))
  (:Started
    (if (Variables|/Script/Engine.Character|GetbIsCrouched _ascharacter)
      (Character|UnCrouch _ascharacter)
      (else
        (Character|Crouch _ascharacter)))))

(event Input|EnhancedActionEvents|EnhancedInputActionIA_Move
  (params (ActionValue :type Vector%202D%20Structure) (ElapsedSeconds :type Float%20%28double-precision%29) (TriggeredSeconds :type Float%20%28double-precision%29) (InputAction :type Input%20Action%20Object%20Reference :default "/Game/_GameManager/Input/IA_Move.IA_Move"))
  (bind _returnvalue (Pawn|GetControlRotation :!class /Script/Engine.Controller))
  (bind _returnvalue_2 (Math|Rotator|MakeRotator (.roll _returnvalue) 0.0 (.yaw _returnvalue)))
  (Pawn|Input|AddMovementInput (Pawn|GetControlledPawn) (Math|Vector|GetForwardVector _returnvalue_2) (.y ActionValue) false) ; forward
  (Pawn|Input|AddMovementInput (Pawn|GetControlledPawn) (Math|Vector|GetRightVector _returnvalue_2) (.x ActionValue) false) ; right
)

(event Input|EnhancedActionEvents|EnhancedInputActionIA_Sprint
  (params (ActionValue :type Boolean) (ElapsedSeconds :type Float%20%28double-precision%29) (TriggeredSeconds :type Float%20%28double-precision%29) (InputAction :type Input%20Action%20Object%20Reference :default "/Game/_GameManager/Input/IA_Sprint.IA_Sprint"))
  (bind _returnvalue (Pawn|GetControlledPawn))
  (bind _returnvalue_2 (Pawn|GetControlledPawn))
  (bind _asbp_base_character (Utilities|Casting|CastToBP_BaseCharacter _returnvalue_2))
  (bind _asbp_base_character_2 (Utilities|Casting|CastToBP_BaseCharacter _returnvalue))
  (:Started
    (Variables|/Script/Engine.CharacterMovementComponent|SetMaxWalkSpeed (Variables|/Script/Engine.Character|GetCharacterMovement _asbp_base_character) (Variables|/Game/_GameManager/BP_BaseCharacter.BP_BaseCharacter_C|GetSprint%20Speed _asbp_base_character)) ; sprint
  )
  (:Completed
    (Variables|/Script/Engine.CharacterMovementComponent|SetMaxWalkSpeed (Variables|/Script/Engine.Character|GetCharacterMovement _asbp_base_character_2) (Variables|/Game/_GameManager/BP_BaseCharacter.BP_BaseCharacter_C|GetRunSpeed _asbp_base_character_2)) ; run
  ))

(event EventPossess
  (params (PossessedPawn :type Pawn%20Object%20Reference))
  (bind _returnvalue (PlayerController|LocalPlayerSubsystems|GetEnhancedInputLocalPlayerSubsystem))
  (Utilities|IsValid _returnvalue
    (:Is%20Valid
      (Input|AddMappingContext _returnvalue "/Game/_GameManager/Input/IMC_Input.IMC_Input" 0 "(bIgnoreAllPressedKeysUntilRelease=True,bForceImmediately=False,bNotifyUserSettings=False)"))))

(fn ConstructionScript)